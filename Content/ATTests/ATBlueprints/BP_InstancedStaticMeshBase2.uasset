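; Base instanced static mesh actor under ATTests that sets up its InstancedStaticMesh component during construction.
; The construction script stores the output of BuildMatrices in Matrices, then calls SetupInstancedMeshComponent with one instance and the AutoPlay setting.
; BuildMatrices here yields a single identity transform matrix.
; A CoordinateAtIndex helper, unused in these graphs, maps an index to an evenly spaced coordinate starting at negative Size.
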(event EventBeginPlay)

(event Collision|EventActorBeginOverlap
  (params (OtherActor :type Actor%20Object%20Reference)))

(event EventTick
  (params (DeltaSeconds :type Float%20%28single-precision%29)))

(fn ConstructionScript
  (bind _outmatrices (CallFunction|BuildMatrices))
  (Variables|Default|SetMatrices _outmatrices)
  (Class|AnimtoTextureInstancePlaybackLibrary|SetupInstancedMeshComponent (Variables|Default|GetInstancedStaticMesh) 1 (Variables|Default|GetAuto%20Play)))

(fn BuildMatrices
  (Utilities|Array|Clear (LocalVariables|Get_Matrices))
  (Utilities|FlowControl|Sequence
    (:then_0
      (Utilities|Array|Add (LocalVariables|Get_Matrices) (Math|Transform|ToMatrix(Transform) (Math|Transform|MakeTransform "0, 0, 0"))))
    (:then_1
      (return (LocalVariables|Get_Matrices)))))

(fn CoordinateatIndex
  (params (Index :type Integer) (Size :type Integer) (Div :type Integer))
  (return (+ (* (Math|Float|MakeLiteralFloat -1.0) Size) (* (Math|Conversions|ToFloat(Integer) Index) (/ (Math|Conversions|ToFloat(Integer) (* Size 2)) (Math|Conversions|ToFloat(Integer) Div))))))