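; Test game mode for an asymmetric match between a Director and a Survivor.
; PostLogin makes the first player the Director, and a later login becomes the Survivor and triggers RoundStart.
; RoundStart spawns and possesses each role's pawn at its start actor, then sets Director mouse input, Survivor HUD and intro sound.
; Logout clears role flags or hands Director to the Survivor if IsSurvivor is set, though this graph never sets it true.
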(event Custom|RoundStart
  (bind _directorplayer (Variables|Default|GetDirectorPlayer))
  (bind _survivorplayer (Variables|Default|GetSurvivorPlayer))
  ;[0.0356 0.0356 0.0356] Round Start
  (Utilities|FlowControl|Sequence
    (:then_0
      (bind _returnvalue (Actor|GetActorOfClass "/Game/Blueprints/Player/BP_DirectorStart.BP_DirectorStart_C"))
      (bind _returnvalue_2 (Game|SpawnActorfromClass "/Game/Blueprints/Player/DirectorPawnTest.DirectorPawnTest_C" (Transformation|GetActorTransform _returnvalue) "Undefined" "MultiplyWithRoot" 0 0))
      (Pawn|Possess _directorplayer _returnvalue_2)
      (Input|SetInputModeGameandUI _directorplayer 0 "LockAlways" true false)
      (Variables|/Script/Engine.PlayerController|SetbShowMouseCursor _directorplayer true))
    (:then_1
      (bind _returnvalue_3 (Actor|GetActorOfClass "/Game/Blueprints/Player/BP_SurvivorStart.BP_SurvivorStart_C"))
      (bind _returnvalue_4 (Game|SpawnActorfromClass "/Game/Blueprints/Player/BP_FirstPersonCharacterMergeTest.BP_FirstPersonCharacterMergeTest_C" (Transformation|GetActorTransform _returnvalue_3) "Undefined" "MultiplyWithRoot" 0 0))
      (Pawn|Possess _survivorplayer _returnvalue_4)
      (Class|PlayerController|ClientSetHUD _survivorplayer "/Game/Misc/BP_SurvivorHUD.BP_SurvivorHUD_C"))
    (:then_2
      (bind _asbp_survivor_controller_merge_test (Utilities|Casting|CastToBP_SurvivorControllerMergeTest (Variables|Default|GetSurvivorPlayer)))
      (Default|SoundSurvivorIntro _asbp_survivor_controller_merge_test))))

(event EventOnLogout
  (params (ExitingController :type Controller%20Object%20Reference))
  ;[0.01938 0.01938 0.01938] Player Disconnect
  (if (== ExitingController (Variables|Default|GetDirectorPlayer))
    (if (Variables|Default|GetIsSurvivor)
      (Variables|Default|SetDirectorPlayer (Variables|Default|GetSurvivorPlayer))
      (Variables|Default|SetIsSurvivor false)
      (else
        (Variables|Default|SetIsDirector false)))
    (else
      (Variables|Default|SetIsSurvivor false))))

(event EventPostLogin
  (params (NewPlayer :type Player%20Controller%20Object%20Reference))
  ;[0.01938 0.01938 0.01938] Player Connect
  (if (Variables|Default|GetIsDirector)
    (Variables|Default|SetSurvivorPlayer NewPlayer)
    (CallFunction|RoundStart)
    (else
      (Variables|Default|SetIsDirector true)
      (Variables|Default|SetDirectorPlayer NewPlayer))))

(fn ConstructionScript)